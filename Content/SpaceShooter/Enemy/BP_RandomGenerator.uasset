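; BP_RandomGenerator is the enemy spawner for the space shooter, spawning enemies on a looping timer started at BeginPlay.
; Each tick picks a random enemy class, bounded by game mode Level and MaxNumEnemies, and a random SceneComponent tagged SpawnPoints.
; Each enemy's destroy event decrements SpawnTime, but the running timer is never reset to use it.
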(event Custom|Spawn
  (bind _enemy_spawned (CallFunction|SpawnEnemy))
  (EventDispatchers|BindEventtoOnEnemyDestroy _enemy_spawned (delegate Custom|EnemyDestroy)))

(event Custom|EnemyDestroy
  (Variables|Default|SetSpawnTime (- (Variables|Default|GetSpawnTime) 1.0)))

(event EventBeginPlay
  (Utilities|Time|SetTimerbyEvent (delegate Custom|Spawn) (Variables|Default|GetSpawnTime) true)
  (bind _asss_game_mode (Utilities|Casting|CastToSS_GameMode (Game|GetGameMode)))
  (Variables|Default|Setm_GameModeR _asss_game_mode))

(fn ConstructionScript)

(fn SpawnEnemy
  (bind _returnvalue (Actor|GetComponentsbyTag "/Script/Engine.SceneComponent" "SpawnPoints"))
  (bind _class (CallFunction|GetClasstoSpawn (Math|Random|RandomInteger (Variables|/Game/SpaceShooter/SS_GameMode.SS_GameMode_C|GetLevel (Variables|Default|Getm_GameModeR)))))
  (bind _returnvalue_2 (Game|SpawnActorfromClass _class (Transformation|GetWorldTransform (Utilities|Array|Get(acopy) _returnvalue (Math|Random|RandomInteger (Utilities|Array|Length _returnvalue)))) "Undefined" "MultiplyWithRoot" 0 0))
  (bind _asbp_enemy_base (Utilities|Casting|CastToBP_EnemyBase _returnvalue_2))
  (return _asbp_enemy_base))

(fn GetClasstoSpawn
  (params (Type :type Integer))
  (return (Utilities|Select :Index (Math|Integer|Clamp(Integer) Type 0 (- (Variables|Default|GetMaxNumEnemies) 1)) :Option%200 "/Game/SpaceShooter/Enemy/BP_EnemyBase.BP_EnemyBase_C" :Option%201 "/Game/SpaceShooter/Enemy/BP_Enemy2.BP_Enemy2_C" :Option%202 0)))