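; BP_Enemy2 is a space shooter enemy that reverses sideways direction whenever it overlaps an actor tagged "Lateral".
; It starts along its right vector, and an IsRight flag flips MovementVector between that vector and its negation.
; Each turn toward negative right also shortens DelayShoot, with no lower limit in this Blueprint.
; BeginPlay, overlap and Tick call the parent; no movement or firing is implemented here.
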(event EventBeginPlay
  (|CallParentFunction)
  (Variables|Default|SetMovementVector (Transformation|GetActorRightVector))
  (Variables|Default|SetIsRight false))

(event EventTick
  (params (DeltaSeconds :type Float%20%28single-precision%29))
  (|CallParentFunction DeltaSeconds))

(event Collision|EventActorBeginOverlap
  (params (OtherActor :type Actor%20Object%20Reference))
  (bind _returnvalue (Transformation|GetActorRightVector))
  (|CallParentFunction OtherActor)
  (if (Utilities|Array|ContainsItem (Variables|/Script/Engine.Actor|GetTags OtherActor) "Lateral")
    (if (Variables|Default|GetIsRight)
      (Variables|Default|SetIsRight false)
      (Variables|Default|SetMovementVector _returnvalue)
      (else
        (Variables|Default|SetIsRight true)
        (Variables|Default|SetMovementVector (Math|Vector|NegateVector _returnvalue))
        (Variables|Default|SetDelayShoot (- (Variables|Default|GetDelayShoot) 0.1))))))

(fn ConstructionScript
  (|CallParentFunction))