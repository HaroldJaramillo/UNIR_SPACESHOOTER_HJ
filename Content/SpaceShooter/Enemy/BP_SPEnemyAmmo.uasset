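; BP_SPEnemyAmmo is an enemy projectile for the space shooter that damages the player on contact.
; Tick moves it along its forward vector at Speed, without sweeping.
; The Sphere overlap applies damage to a BP_SpaceS_Character and destroys the projectile at once.
; Actor overlap with any non-Pawn spawns an explosion effect and sound, then destroys it after a short delay.
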(event OnComponentBeginOverlap(Sphere)
  (params (OverlappedComponent :type Primitive%20Component%20Object%20Reference) (OtherActor :type Actor%20Object%20Reference) (OtherComp :type Primitive%20Component%20Object%20Reference) (OtherBodyIndex :type Integer) (bFromSweep :type Boolean) (SweepResult :type Hit%20Result%20Structure%20%28by%20ref%29))
  ;[0.15 0.15 0.15 0.5] Hace daño al jugador
  (bind _asbp_space_s_character (Utilities|Casting|CastToBP_SpaceS_Character OtherActor))
  (Game|Damage|ApplyDamage _asbp_space_s_character 1.0 0 0)
  (Actor|DestroyActor))

(event Collision|EventActorBeginOverlap
  (params (OtherActor :type Actor%20Object%20Reference))
  (Utilities|Casting|CastToPawn OtherActor
    (:CastFailed
      (Effects|SpawnEmitteratLocation "/Game/StarterContent/Particles/P_Explosion.P_Explosion" (Transformation|GetActorLocation))
      (Audio|PlaySound2D "/Game/StarterContent/Audio/Explosion02.Explosion02" 0.05 1.0 0.0 0 0)
      (Utilities|FlowControl|Delay 0.2)
      (Actor|DestroyActor))))

(event EventTick
  (params (DeltaSeconds :type Float%20%28single-precision%29))
  (Transformation|SetActorLocation (+ (Transformation|GetActorLocation) (* (Transformation|GetActorForwardVector) (* DeltaSeconds (Variables|Default|GetSpeed)))) false false))

(fn ConstructionScript)