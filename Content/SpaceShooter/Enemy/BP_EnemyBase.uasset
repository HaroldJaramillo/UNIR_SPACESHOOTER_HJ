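; Base enemy ship for the space shooter that flies along its initial forward vector and fires ammo from its fire point on a timer.
; Overlapping a Player-tagged actor triggers its destroy dispatcher, whose bound event removes it after a short delay.
; It also notifies SS_GameMode and spawns a random coin or power-up at a line trace's hit location.
; The ammo-cast branch into this death logic is unconnected.
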(event Custom|Destroyed_Event
  ;[0.15 0.15 0.15 0.5] El enemigo se mueve
  (Utilities|FlowControl|Delay 0.2)
  (Actor|DestroyActor))

(event Custom|DropLoot
  ;[0.15 0.15 0.15 0.5] El enemigo dropea loot
  (bind _outhit (Collision|LineTraceByChannel (Transformation|GetActorLocation) "0, 0, 0" "TraceTypeQuery1" false 0 "None"))
  (Game|SpawnActorfromClass (Utilities|Select :Index (Math|Random|RandomInteger 3) :Option%200 "/Game/SpaceShooter/Points/BP_Coin1.BP_Coin1_C" :Option%201 "/Game/SpaceShooter/PowerUps/BP_ShootSpeedUp.BP_ShootSpeedUp_C" :Option%202 "/Game/SpaceShooter/PowerUps/BP_SpeedPU.BP_SpeedPU_C") (Math|Transform|MakeTransform (.Location (Collision|BreakHitResult _outhit)) (Math|Rotator|MakeRotator 0.0 0.0 (Math|Random|RandomFloatinRange 0.0 0.0))) "Undefined" "MultiplyWithRoot" 0))

(event EventBeginPlay
  ;[0.15 0.15 0.15 0.5] El enemigo se mueve
  (Variables|Default|SetMovementVector (Transformation|GetActorForwardVector))
  (EventDispatchers|BindEventtoOnEnemyDestroy (delegate Custom|Destroyed_Event)))

(event EventTick
  (params (DeltaSeconds :type Float%20%28single-precision%29))
  ;[0.15 0.15 0.15 0.5] El enemigo dispara
  (CallFunction|Move DeltaSeconds)
  (bind _output_get (Variables|Default|SetShotCurrentTime (+ DeltaSeconds (Variables|Default|GetShotCurrentTime))))
  (if (> _output_get (Variables|Default|GetDelayShoot))
    (Variables|Default|SetShotCurrentTime 0.0)
    (CallFunction|Fire)))

(event Collision|EventActorBeginOverlap
  (params (OtherActor :type Actor%20Object%20Reference))
  ;[0.15 0.15 0.15 0.5] El enemigo muere y arroja loot
  (if (Utilities|Array|ContainsItem (Variables|/Script/Engine.Actor|GetTags OtherActor) "Player")
    (Default|CallOnEnemyDestroy)
    (bind _asss_game_mode (Utilities|Casting|CastToSS_GameMode (Game|GetGameMode)))
    (Default|EnemyDestroyed _asss_game_mode)
    (CallFunction|DropLoot)))

(fn ConstructionScript)

(fn Move
  (params (DeltaTime :type Float%20%28double-precision%29))
  (Transformation|SetActorLocation (+ (Transformation|GetActorLocation) (* (Variables|Default|GetMovementVector) (* DeltaTime (Variables|Default|GetSpeed)))) false false))

(fn Fire
  (bind _returnvalue (Game|SpawnActorfromClass (Variables|Default|GetAmmo) (Transformation|GetWorldTransform (Variables|Default|GetFirePoint)) "Undefined" "MultiplyWithRoot" 0 0))
  (Transformation|SetActorRotation _returnvalue (Transformation|GetActorRotation)))