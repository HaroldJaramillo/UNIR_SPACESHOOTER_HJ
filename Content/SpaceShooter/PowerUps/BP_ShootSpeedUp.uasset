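; BP_ShootSpeedUp is a space shooter pickup that increases the player's shooting speed when a BP_SpaceS_Character overlaps it, then destroys itself.
; On BeginPlay, two timers limit its lifetime: one destroys it after LifeTime, the other starts blinking BlinkTime earlier.
; Blinking uses a looping timer that toggles the Powerup component's visibility every BlinkInterval to signal the coming expiry.
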(event Custom|StartBlinking
  (Utilities|Time|SetTimerbyEvent (delegate Custom|ToggleVisibility) (Variables|Default|GetBlinkInterval) true))

(event Custom|ToggleVisibility
  (Variables|Default|SetIsVisible (not (Variables|Default|GetIsVisible)))
  (Rendering|SetVisibility (Variables|Default|Getpower-up) (Variables|Default|GetIsVisible) false))

(event Custom|DestroySelf
  (Actor|DestroyActor))

(event EventBeginPlay
  (Utilities|FlowControl|Sequence
    (:then_0
      (Utilities|Time|SetTimerbyEvent (delegate Custom|StartBlinking) (- (Variables|Default|GetLifeTime) (Variables|Default|GetBlinkTime))))
    (:then_1
      (Utilities|Time|SetTimerbyEvent (delegate Custom|DestroySelf) (Variables|Default|GetLifeTime)))))

(event Collision|EventActorBeginOverlap
  (params (OtherActor :type Actor%20Object%20Reference))
  (bind _asbp_space_s_character (Utilities|Casting|CastToBP_SpaceS_Character OtherActor))
  (Default|IncreasseShootSpeed _asbp_space_s_character)
  (Actor|DestroyActor))

(event EventTick
  (params (DeltaSeconds :type Float%20%28single-precision%29)))

(fn ConstructionScript)