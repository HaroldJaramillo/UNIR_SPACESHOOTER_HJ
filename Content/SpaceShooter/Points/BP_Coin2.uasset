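; BP_Coin2 is a timed coin pickup for the space shooter that awards score to the player and expires if left uncollected.
; On BeginPlay, timers start a looping mesh visibility blink shortly before the lifetime ends, then destroy the actor.
; When the player character overlaps its sphere, it plays a coin sound, adds a fixed amount to the Game Instance score and destroys itself.
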(event OnComponentBeginOverlap(Sphere)
  (params (OverlappedComponent :type Primitive%20Component%20Object%20Reference) (OtherActor :type Actor%20Object%20Reference) (OtherComp :type Primitive%20Component%20Object%20Reference) (OtherBodyIndex :type Integer) (bFromSweep :type Boolean) (SweepResult :type Hit%20Result%20Structure%20%28by%20ref%29))
  (bind _asbp_space_s_character (Utilities|Casting|CastToBP_SpaceS_Character OtherActor))
  (Utilities|IsValid _asbp_space_s_character
    (:Is%20Valid
      (Audio|PlaySound2D "/Game/SpaceShooter/Points/COIN_SOUND.COIN_SOUND" 1.0 1.0 0.0 0 0)
      (bind _asbp_my_game_instance (Utilities|Casting|CastToBP_MyGameInstance (Game|GetGameInstance)))
      (Variables|/Game/SpaceShooter/Points/BP_MyGameInstance.BP_MyGameInstance_C|SetScore _asbp_my_game_instance (+ (Variables|/Game/SpaceShooter/Points/BP_MyGameInstance.BP_MyGameInstance_C|GetScore _asbp_my_game_instance) 20))
      (Actor|DestroyActor))))

(event Custom|StartBlinking
  (Utilities|Time|SetTimerbyEvent (delegate Custom|ToggleVisibility) (Variables|Default|GetBlinkInterval) true))

(event Custom|ToggleVisibility
  (Variables|Default|SetIsVisible (not (Variables|Default|GetIsVisible)))
  (Rendering|SetVisibility (Variables|Default|GetStaticMesh) (Variables|Default|GetIsVisible) false))

(event Custom|DestroySelf
  (Actor|DestroyActor))

(event EventBeginPlay
  (Utilities|FlowControl|Sequence
    (:then_0
      (Utilities|Time|SetTimerbyEvent (delegate Custom|StartBlinking) (- (Variables|Default|GetLifeTime) (Variables|Default|GetBlinkTime))))
    (:then_1
      (Utilities|Time|SetTimerbyEvent (delegate Custom|DestroySelf) (Variables|Default|GetLifeTime)))))

(fn ConstructionScript)